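; BP_SpawnAndDestroyAxis toggles a BP_CoordinateAxis actor in and out of the world.
; SpawnAndDestroy checks IsSpawned, then either spawns the axis at the world origin and stores it in TargetActor, or destroys the stored actor.
; Both branches show the mouse cursor and print a debug message.
; The BeginPlay input setup and Z key trigger are disabled, so nothing in this Blueprint calls the toggle.
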(event EventBeginPlay
  (Input|EnableInput (Game|GetPlayerController 0)))

(event Input|KeyboardEvents|Z
  (params (Key :type Key%20Structure :default "None"))
  (:Pressed
    (CallFunction|SpawnandDestroy)))

(fn ConstructionScript)

(fn SpawnandDestroy
  ;[1 1 1] Spawn the coordinate axis when it needs to be used ;
  ; Destroy it when it is not used.
  (if (Variables|Default|Getis%20spawned)
    (Actor|DestroyActor (Variables|Default|GetTargetActor))
    (Variables|/Script/Engine.PlayerController|SetbShowMouseCursor (Game|GetPlayerController 0) true)
    (Variables|Default|Setis%20spawned false)
    (Development|PrintString "Aixs Destroy" true false "(R=0.000000,G=0.660000,B=1.000000,A=1.000000)" 1e+01)
    (else
      (bind _returnvalue (Game|SpawnActorfromClass "/Game/Blueprints/CoordinateAxis/Axis/Blueprints/BP_CoordinateAxis.BP_CoordinateAxis_C" (Math|Transform|MakeTransform "0, 0, 0") "Undefined" 0 0))
      (Variables|Default|SetTargetActor _returnvalue)
      (Variables|/Script/Engine.PlayerController|SetbShowMouseCursor (Game|GetPlayerController 0) true)
      (Variables|Default|Setis%20spawned true)
      (Development|PrintString "Aixs Spawn" true false "(R=0.000000,G=0.660000,B=1.000000,A=1.000000)" 1e+01))))