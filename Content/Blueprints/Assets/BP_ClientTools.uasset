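; Client-only tool actor that switches click-through on or off based on whether content is under the mouse.
; It destroys itself on dedicated servers; elsewhere BeginPlay sets a short, non-looping timer for the mouse check.
; The check compares the result with its cached value and calls SetClickThrough only on a change, disabling click-through over content.
; As wired, the timer fires only once, so the check does not repeat.
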(event Custom|CheckForContentUnderMouse
  (bind _returnvalue (Class|WindowTransparencyBPFunctionLibrary|HasContentUnderMouse))
  (if (Math|Boolean|Equal(Boolean) _returnvalue (Variables|Default|GetLastContentUnderMouse))
    (Variables|Default|SetLastContentUnderMouse _returnvalue)
    (else
      (Variables|Default|SetLastContentUnderMouse _returnvalue)
      (if _returnvalue
        (Class|WindowTransparencyBPFunctionLibrary|SetClickThrough false)
        (else
          (Class|WindowTransparencyBPFunctionLibrary|SetClickThrough true))))))

(event EventBeginPlay
  ;[1 1 1] this tool only runs on clients
  (if (Networking|IsDedicatedServer)
    (Actor|DestroyActor)
    (else
      (Utilities|Time|SetTimerbyEvent (delegate Custom|CheckForContentUnderMouse) 0.05))))

(event Collision|EventActorBeginOverlap
  (params (OtherActor :type Actor%20Object%20Reference)))

(event EventTick
  (params (DeltaSeconds :type Float%20%28single-precision%29)))

(fn ConstructionScript)