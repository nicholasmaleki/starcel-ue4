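; BP_PyActor is a utility actor wrapping engine calls as events: window mode, transparency, desktop-background window, global time dilation and Python string execution.
; Python execution is noted to work only when the actor is server-spawned.
; ConvertImageToCubemap starts an async runtime HDRI load, storing the texture and success flag; GetCubemap returns the texture.
; An authority-checked event spawns a LargeStringRPCActor owned by the first player controller, but its automatic trigger is disconnected.
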(event Custom|EventRunBlueprintFunctions
  (Utilities|Time|SetGlobalTimeDilation (Variables|Default|GetTimeDilation)))

(event Custom|ConvertImageToCubemapEvent
  (params (texture2d :type String))
  (bind (_outtexturecube _bsuccess) (Class|RuntimeImageLoader|LoadHDRIasCubemapAsync (Subsystems|GetRuntimeImageLoader) texture2d))
  (Variables|Default|SetTextureCube _outtexturecube)
  (Variables|Default|SetCubemapFinished _bsuccess))

(event Custom|SpawnRPCActorOnServer
  (Networking|SwitchHasAuthority
    (:Authority
      (Game|SpawnActorfromClass "/Script/LargeData.LargeStringRPCActor" (Math|Transform|MakeTransform "0, 0, 0" "0, 0, 0" "1,1,1") "Undefined" (Game|GetPlayerController 0) 0))
    (:Remote
      (Development|PrintString "No authority to spawn the large string rpc actor"))))

(event Custom|SetWindowTransparent
  (Class|WindowTransparencyBPFunctionLibrary|EnableWindowTransparency true))

(event Custom|DisableWindowTransparent
  (Class|WindowTransparencyBPFunctionLibrary|DisableWindowTransparency))

(event Custom|SetFullscreen
  (bind _returnvalue (Settings|GetGameUserSettings))
  (Class|GameUserSettings|SetFullscreenMode _returnvalue "Fullscreen"))

(event Custom|SetWindowed
  (bind _returnvalue (Settings|GetGameUserSettings))
  (Class|GameUserSettings|SetFullscreenMode _returnvalue "Windowed"))

(event Custom|RestoreFromDesktopBackground
  (Class|WindowTransparencyBPFunctionLibrary|RestorefromDesktopBackground))

(event Custom|SetWindowedFullscreen
  (bind _returnvalue (Settings|GetGameUserSettings))
  (Class|GameUserSettings|SetFullscreenMode _returnvalue "WindowedFullscreen"))

(event Custom|SetWindowAsDesktopBackground
  (Class|WindowTransparencyBPFunctionLibrary|SetasDesktopBackground))

(event Custom|RunPythonOnServer
  (params (NewParam :type String))
  ;[1 1 1] only works if the pyactor is spawned on the server
  (Class|PythonBlueprintFunctionLibrary|ExecutePythonString NewParam))

(event EventBeginPlay)

(event Collision|EventActorBeginOverlap
  (params (OtherActor :type Actor%20Object%20Reference)))

(event EventTick
  (params (DeltaSeconds :type Float%20%28single-precision%29)))

(fn ConstructionScript)

(fn ConvertImagetoCubemap
  (params (file%20path :type String))
  (CallFunction|ConvertImagetoCubemapEvent file%20path)
  (return))

(fn GetCubemap
  (return (Variables|Default|GetTextureCube)))