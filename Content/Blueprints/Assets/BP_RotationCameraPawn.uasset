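; Camera pawn that slowly yaws its Scene component, apparently to orbit the view around a person.
; BeginPlay prints the owner's name and runs a console command for Panini projection and screen percentage.
; Tick eases the yaw toward a full negative turn with a very low-speed FInterpTo and applies it as world rotation.
; A similar pitch interpolation is left disconnected and never runs.
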(event EventBeginPlay
  (Development|PrintString (Utilities|GetDisplayName (Components|GetOwner)))
  (Development|ExecuteConsoleCommand "r.Upscale.Panini.D 0.5 | r.Upscale.Panini.S 0.05 | r.ScreenPercentage 150" (Game|GetPlayerController 0)))

(event Collision|EventActorBeginOverlap
  (params (OtherActor :type Actor%20Object%20Reference)))

(event EventTick
  (params (DeltaSeconds :type Float%20%28single-precision%29))
  (bind _output_get (Variables|Default|SetRotAroundPerson (Math|Interpolation|FInterpTo (Variables|Default|GetRotAroundPerson) -3.6e+02 (Utilities|Time|GetWorldDeltaSeconds) 0.0001)))
  (Transformation|SetWorldRotation (Variables|Default|GetScene) (Math|Rotator|MakeRotator 0.0 0.0 _output_get) false false))

(fn ConstructionScript)