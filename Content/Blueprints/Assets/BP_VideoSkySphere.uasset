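; BP_VideoSkySphere is a sky sphere actor that plays a video background through a media player.
; SetVideoBackground opens the given path as a URL on the MediaPlayer.
; An OnMediaOpened handler restarts playback from zero with debug prints, but its binding is unconnected.
; Older stream-texture and dynamic material setup on the static mesh is left disabled, and BeginPlay, Tick and construction are empty.
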(event Custom|SetVideoBackground
  (params (path :type String))
  (Class|MediaPlayer|OpenUrl (Variables|Default|GetMedia%20Player) path))

(event Custom|OnMediaOpened_Event_0
  (params (OpenedUrl :type String))
  (bind _media_player (Variables|Default|GetMedia%20Player))
  (Development|PrintString "run")
  (Sequencer|Player|Pause _media_player)
  (Media|MediaPlayer|Seek _media_player (Math|Timespan|MakeTimespan 0))
  (Media|MediaPlayer|Play _media_player :!class /Script/MediaAssets.MediaPlayer)
  (Development|PrintString "finished"))

(event EventBeginPlay)

(event Collision|EventActorBeginOverlap
  (params (OtherActor :type Actor%20Object%20Reference)))

(event EventTick
  (params (DeltaSeconds :type Float%20%28single-precision%29)))

(fn ConstructionScript)