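; BP_DroneCharacter is a drone character Blueprint that keeps a Screen component sized to fill its camera view.
; Each Tick, outside dedicated servers and with a valid player pawn, it derives width from camera FOV and ScreenSpringArm length, and height from the viewport aspect ratio.
; The result becomes the Screen's world scale, with a near-flat depth.
; BeginPlay only checks the player pawn and does nothing further.
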(event EventBeginPlay
  (Utilities|IsValid (Game|Player|GetPlayerPawn 0)))

(event Collision|EventActorBeginOverlap
  (params (OtherActor :type Actor%20Object%20Reference)))

(event EventTick
  (params (DeltaSeconds :type Float%20%28single-precision%29))
  (bind _returnvalue (Viewport|GetViewportSize))
  (bind _camera (Variables|Default|GetCamera))
  (bind _screenspringarm (Variables|Default|GetScreenSpringArm))
  (bind (_x _y) (Math|Vector2D|BreakVector2D _returnvalue))
  (bind _fieldofview (Variables|/Script/Engine.CameraComponent|GetFieldOfView _camera))
  (bind _targetarmlength (Variables|/Script/Engine.SpringArmComponent|GetTargetArmLength _screenspringarm))
  (bind _returnvalue_2 (Math|Trig|DegreesToRadians _fieldofview))
  (bind _returnvalue_3 (/ _returnvalue_2 2.0))
  (bind _returnvalue_4 (Math|Trig|Tan(Radians) _returnvalue_3))
  (bind _returnvalue_5 (* _returnvalue_4 _targetarmlength 2.0))
  (Utilities|IsValid (Game|Player|GetPlayerPawn 0)
    (:Is%20Valid
      (if (not (Networking|IsDedicatedServer))
        (Transformation|SetWorldScale3D (Variables|Default|GetScreen) (* (/ (Math|Vector|MakeVector 0.01 _returnvalue_5 (* (/ _y _x) _returnvalue_5)) 1e+02) 1.0))))))

(fn ConstructionScript)